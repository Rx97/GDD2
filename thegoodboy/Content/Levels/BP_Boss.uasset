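; Boss actor that fires at the player and advances through damage-based stages until opening the victory level.
; Tick yaws the body and three spawn points toward the player and checks health lost against stage thresholds.
; Each stage change swaps the mesh, explodes, disables boss and player shooting, flags the player's transition, spawns a platform and, after a delay, activates game mode spawners.
; Shoot fires three projectiles, re-calling itself after a delay.
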(event `Shoot`
  (if (`self.CanShoot`)
    (`|SpawnActorFromClass` "/Game/FirstPersonBP/Blueprints/FirstPersonProjectile.FirstPersonProjectile_C" (`SceneComponent.K2_GetComponentToWorld` (`self.SpawnPoint1`)) "Undefined" "OverrideRootScale" null null)
    (`|SpawnActorFromClass` "/Game/FirstPersonBP/Blueprints/FirstPersonProjectile.FirstPersonProjectile_C" (`SceneComponent.K2_GetComponentToWorld` (`self.SpawnPoint2`)) "Undefined" "OverrideRootScale" null null)
    (`|SpawnActorFromClass` "/Game/FirstPersonBP/Blueprints/FirstPersonProjectile.FirstPersonProjectile_C" (`SceneComponent.K2_GetComponentToWorld` (`self.SpawnPoint3`)) "Undefined" "OverrideRootScale" null null)
    (`KismetSystemLibrary.Delay` (`self.ShootDelay`))
    (`self.Shoot`)))

(event `self.ReceiveTick`
  (params (DeltaSeconds :type "Float (single-precision)"))
  (bind (_returnvalue_roll _returnvalue_pitch) (`KismetMathLibrary.BreakRotator` (`self.K2_GetActorRotation`)))
  (bind _returnvalue (`GameplayStatics.GetPlayerCharacter` 0))
  (bind _spawnpoint2 (`self.SpawnPoint2`))
  (bind _spawnpoint3 (`self.SpawnPoint3`))
  (bind _spawnpoint1 (`self.SpawnPoint1`))
  (bind (_returnvalue_roll_2 _returnvalue_pitch_2) (`KismetMathLibrary.BreakRotator` (`SceneComponent.K2_GetComponentRotation` _spawnpoint1)))
  (bind (_returnvalue_roll_3 _returnvalue_pitch_3) (`KismetMathLibrary.BreakRotator` (`SceneComponent.K2_GetComponentRotation` _spawnpoint2)))
  (bind (_returnvalue_roll_4 _returnvalue_pitch_4) (`KismetMathLibrary.BreakRotator` (`SceneComponent.K2_GetComponentRotation` _spawnpoint3)))
  (bind _asfirst_person_character (cast `/Game/FirstPersonBP/Blueprints/FirstPersonCharacter` (`GameplayStatics.GetPlayerCharacter` 0) :!pure true))
  (`/Engine/EditorBlueprintResources/StandardMacros.IsValid` _returnvalue
    (:`Is Valid`
      (`|ExecutionSequence`
        (:`then_0`
          (`self.K2_SetActorRotation` (`KismetMathLibrary.MakeRotator` _returnvalue_roll _returnvalue_pitch (- (.yaw (`KismetMathLibrary.FindLookAtRotation` (`self.K2_GetActorLocation`) (`self.K2_GetActorLocation` _returnvalue))) 90.0)))
          (`SceneComponent.K2_SetWorldRotation` _spawnpoint1 (`KismetMathLibrary.MakeRotator` _returnvalue_roll_2 _returnvalue_pitch_2 (.yaw (`KismetMathLibrary.FindLookAtRotation` (`SceneComponent.K2_GetComponentLocation` (`self.SpawnPoint1`)) (`self.K2_GetActorLocation` (`GameplayStatics.GetPlayerCharacter` 0))))) false false)
          (`SceneComponent.K2_SetWorldRotation` _spawnpoint2 (`KismetMathLibrary.MakeRotator` _returnvalue_roll_3 _returnvalue_pitch_3 (.yaw (`KismetMathLibrary.FindLookAtRotation` (`SceneComponent.K2_GetComponentLocation` (`self.SpawnPoint2`)) (`self.K2_GetActorLocation` (`GameplayStatics.GetPlayerCharacter` 0))))) false false)
          (`SceneComponent.K2_SetWorldRotation` _spawnpoint3 (`KismetMathLibrary.MakeRotator` _returnvalue_roll_4 _returnvalue_pitch_4 (.yaw (`KismetMathLibrary.FindLookAtRotation` (`SceneComponent.K2_GetComponentLocation` (`self.SpawnPoint3`)) (`self.K2_GetActorLocation` (`GameplayStatics.GetPlayerCharacter` 0))))) false false))
        (:`then_1`
          (if (>= (- (`self.MaxHealth`) (`self.CurrentHealth`)) (`KismetMathLibrary.Conv_IntToDouble` (* (`self.StageNumber`) 15)))
            (if (< (`self.StageNumber`) 3)
              (`/Engine/EditorBlueprintResources/StandardMacros.IncrementInt` (`self.StageNumber`)
                (:`  `
                  (set `/Game/FirstPersonBP/Blueprints/FirstPersonCharacter.TransitionBack` true _asfirst_person_character)
                  (set `/Game/FirstPersonBP/Blueprints/FirstPersonCharacter.CanShoot` false _asfirst_person_character)
                  (`StaticMeshComponent.SetStaticMesh` (`self.StaticMeshComponent`) (`|GetArrayItem` (`self.Stages`) (- (`self.StageNumber`) 1)))
                  (set `/Game/FirstPersonBP/Blueprints/FirstPersonCharacter.StartingPosition` (`self.GetTransform` _asfirst_person_character) _asfirst_person_character)
                  (`GameplayStatics.SpawnEmitterAtLocation` "/Game/StarterContent/Particles/P_Explosion.P_Explosion" (`SceneComponent.K2_GetComponentLocation` (`self.StaticMeshComponent`)) (struct) (100.0 100.0 100.0))
                  (set `self.CanShoot` false)
                  (bind _returnvalue_2 (`|SpawnActorFromClass` "/Game/PlatformTesting/Platform.Platform_C" (`KismetMathLibrary.MakeTransform` (-1000.0 0.0 900.0) (struct :`Yaw` 180.0) (100.0 24.0 8.0)) "Undefined" "OverrideRootScale" null null))
                  (set `/Game/PlatformTesting/Platform.Travel Distance` 15000.0 _returnvalue_2)
                  (`KismetSystemLibrary.Delay` 3.0)
                  (for _array_element (`/Game/FirstPersonBP/Blueprints/FirstPersonGameMode.Spawners` (cast `/Game/FirstPersonBP/Blueprints/FirstPersonGameMode` (`GameplayStatics.GetGameMode`) :!pure true))
                    (set `/Game/PlatformTesting/PlatformSpawner.IsSpawning` true _array_element))))
              (else
                (`GameplayStatics.OpenLevel` "Victory_Level")))))))))

(fn `UserConstructionScript`)