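; BP_FireballSpawner is a test actor that repeatedly launches batches of FirstPersonProjectile as fireballs across an area of the level.
; After a short delay on BeginPlay, ShootFireballs spawns ten projectiles at random X/Y world positions at a fixed height, each with a random upward pitch.
; The event then waits and calls itself again, repeating indefinitely; spawn positions ignore the spawner's own location.
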(event `self.ReceiveBeginPlay`
  (`KismetSystemLibrary.Delay` 3.0)
  (`self.ShootFireballs`))

(event `ShootFireballs`
  (for _ (range 10)
    (`|SpawnActorFromClass` "/Game/FirstPersonBP/Blueprints/FirstPersonProjectile.FirstPersonProjectile_C" (`KismetMathLibrary.MakeTransform` (`KismetMathLibrary.MakeVector` (`KismetMathLibrary.RandomFloatInRange` -2500.0 2500.0) (`KismetMathLibrary.RandomFloatInRange` -1500.0 1500.0) 225.0) (`KismetMathLibrary.MakeRotator` 0.0 (`KismetMathLibrary.RandomFloatInRange` 30.0 150.0))) "Undefined" "OverrideRootScale" null null))
  (`KismetSystemLibrary.Delay` 5.0)
  (`self.ShootFireballs`))

(fn `UserConstructionScript`)