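; Coin shop actor that tracks a coin count against a required amount, showing progress through world text and a point light colored red or green.
; Other code feeds coins in through AddCoin, which refreshes the display.
; An interact box shows a turn-in prompt and enables E input for the player character once enough coins are held.
; Turning in subtracts the cost and asks FirstPersonGameMode to create a new shop.
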(event `self.ReceiveBeginPlay`
  (`self.Update Text`))

(event `Key|E`
  (params (Key :type "Key Structure"))
  (:`Pressed`
    (`self.TurnInCoins`)))

(event `AddCoin`
  (`/Engine/EditorBlueprintResources/StandardMacros.IncrementInt` (`self.CoinCount`)
    (:`  `
      (`self.Update Text`))))

(event `TurnInCoins`
  (if (>= (`self.CoinCount`) (`self.CoinsNeeded`))
    (set `self.CoinCount` (- (`self.CoinCount`) (`self.CoinsNeeded`)))
    (`self.Update Text`)
    (bind _asfirst_person_game_mode (cast `/Game/FirstPersonBP/Blueprints/FirstPersonGameMode` (`GameplayStatics.GetGameMode`)))
    (`/Game/FirstPersonBP/Blueprints/FirstPersonGameMode.CreateNewShop` _asfirst_person_game_mode (`self.CoinCount`) (`self.CoinsNeeded`))))

(event `Update Text`
  (`TextRenderComponent.K2_SetText` (`self.CoinCountText`) (`KismetTextLibrary.Conv_StringToText` (`KismetStringLibrary.BuildString_Int` (`KismetStringLibrary.Conv_IntToString` (`self.CoinCount`)) "/" (`self.CoinsNeeded`) " Coins")))
  (if (>= (`self.CoinCount`) (`self.CoinsNeeded`))
    (`LightComponent.SetLightColor` (`self.PointLight`) (struct :`G` 1.0 :`A` 1.0) true)
    (`TextRenderComponent.SetTextRenderColor` (`self.CoinCountText`) (`KismetMathLibrary.Conv_LinearColorToColor` (struct :`G` 1.0 :`A` 1.0)))
    (else
      (`LightComponent.SetLightColor` (`self.PointLight`) (struct :`R` 1.0 :`A` 1.0) true)
      (`TextRenderComponent.SetTextRenderColor` (`self.CoinCountText`) (`KismetMathLibrary.Conv_LinearColorToColor` (struct :`R` 1.0 :`A` 1.0)))))
  (if (not (>= (`self.CoinCount`) (`self.CoinsNeeded`)))
    (`SceneComponent.SetHiddenInGame` (`self.TurnInText`) true false)))

(event `self.InteractBox.OnComponentBeginOverlap`
  (params (OverlappedComponent :type "PrimitiveComponent Object Reference") (OtherActor :type "Actor Object Reference") (OtherComp :type "PrimitiveComponent Object Reference") (OtherBodyIndex :type Integer) (bFromSweep :type Boolean) (SweepResult :type "HitResult Structure (by ref)"))
  (cast `/Game/FirstPersonBP/Blueprints/MyFirstPersonCharacter` OtherActor)
  (if (>= (`self.CoinCount`) (`self.CoinsNeeded`))
    (`SceneComponent.SetHiddenInGame` (`self.TurnInText`) false false)
    (`self.EnableInput` (`GameplayStatics.GetPlayerController` 0))))

(event `self.InteractBox.OnComponentEndOverlap`
  (params (OverlappedComponent :type "PrimitiveComponent Object Reference") (OtherActor :type "Actor Object Reference") (OtherComp :type "PrimitiveComponent Object Reference") (OtherBodyIndex :type Integer))
  (cast `/Game/FirstPersonBP/Blueprints/MyFirstPersonCharacter` OtherActor)
  (`SceneComponent.SetHiddenInGame` (`self.TurnInText`) true false)
  (`self.DisableInput` (`GameplayStatics.GetPlayerController` 0)))

(fn `UserConstructionScript`)